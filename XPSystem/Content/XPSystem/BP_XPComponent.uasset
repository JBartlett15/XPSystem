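; BP_XPComponent is an XP component that holds a Stats array and sets up an XP bar display.
; On BeginPlay it creates WBP_XPBars, adds the same UIRef to its scroll box once per stat with debug prints, then shows it.
; UpdateUI is empty and uncalled; its disconnected logic would level up the current stat and refresh name, level, XP text and progress bar.
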(event `self.ReceiveBeginPlay`
  (bind _returnvalue (`|CreateWidget` "/Game/XPSystem/WBP_XPBars.WBP_XPBars_C"))
  (set `self.UI` _returnvalue)
  (for _index (range 1 (+ (`KismetArrayLibrary.Array_Length` (`self.Stats`)) 1))
    (`PanelWidget.AddChild` (`/Game/XPSystem/WBP_XPBars.ScrollBox` (`self.UI`)) (`self.UIRef`))
    (`KismetSystemLibrary.PrintString` (`KismetStringLibrary.Conv_IntToString` _index)))
  (`KismetSystemLibrary.PrintString` "Completed")
  (`UserWidget.AddToViewport` (`self.UI`) 0))

(event `self.ReceiveTick`
  (params (DeltaSeconds :type "Float (single-precision)")))

(fn `UpdateUI`)